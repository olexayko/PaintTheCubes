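; BP_TargetCube is a cube actor that spreads or clears player paint when it hits another target cube.
; On Hit, a non-purifier cube struck by a Purifier cube resets to the default target material.
; A player-painted cube passes its material to a default-colored cube it hits, using the current material as its state.
; Either rule calls TryEndGame after changing a material.
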(event EventBeginPlay)

(event Collision|EventActorBeginOverlap
  (params (OtherActor :type Actor%20Object%20Reference)))

(event EventTick
  (params (DeltaSeconds :type Float%20%28single-precision%29)))

(event Collision|EventHit
  (params (MyComp :type Primitive%20Component%20Object%20Reference) (Other :type Actor%20Object%20Reference) (OtherComp :type Primitive%20Component%20Object%20Reference) (bSelfMoved :type Boolean) (HitLocation :type Vector :default "0, 0, 0") (HitNormal :type Vector :default "0, 0, 0") (NormalImpulse :type Vector :default "0, 0, 0") (Hit :type Hit%20Result%20Structure%20%28by%20ref%29))
  (bind _asbp_target_cube (Utilities|Casting|CastToBP_TargetCube Other))
  (Utilities|FlowControl|Sequence
    (:then_0
      ;[1 1 1] Set default target material to purifier if purifier collides with target
      (if (and (Variables|/Script/PaintTheCubes.TargetCube|GetbPurifier _asbp_target_cube) (not (Variables|Default|GetbPurifier)))
        (bind _materialinterface (CallFunction|GetTargetDefaultColor))
        (Rendering|Material|SetMaterial (Variables|Default|GetCube) 0 _materialinterface)
        (CallFunction|TryEndGame :!label _label)))
    (:then_1
      ;[1 1 1] Set default target material to cube if it collides with target painted by player
      (bind _materialinterface_2 (CallFunction|GetPlayerDefaultColor))
      (bind _materialinterface_3 (CallFunction|GetTargetDefaultColor))
      (if (and (== (Rendering|Material|GetMaterial (Variables|Default|GetCube) 0) _materialinterface_2) (== (Rendering|Material|GetMaterial (Variables|BP_TargetCube_C|GetCube _asbp_target_cube) 0) _materialinterface_3))
        (Rendering|Material|SetMaterial (Variables|BP_TargetCube_C|GetCube _asbp_target_cube) 0 _materialinterface_2)
        (goto _label)))))

(fn ConstructionScript)