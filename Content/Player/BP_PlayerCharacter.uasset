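; Player character that moves around the level and paints target cubes with its sphere's material on hit.
; Enhanced Input drives movement along flattened camera-to-capsule vectors, with spring-arm yaw, clamped pitch and a debug velocity arrow.
; Hitting a cube clears its Purifier flag, updates the UI widget created at BeginPlay, plays a pop sound and calls TryEndGame.
; The construction script applies the default player color to the sphere.
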(event Custom|On%20Hit%20Target%20Cube
  (Default|UpdateUI (Variables|Default|GetUi)))

(event Input|EnhancedActionEvents|EnhancedInputActionIA_Move
  (params (ActionValue :type Vector%202D%20Structure) (ElapsedSeconds :type Float%20%28double-precision%29) (TriggeredSeconds :type Float%20%28double-precision%29) (InputAction :type Input%20Action%20Object%20Reference :default "/Game/Input/IA_Move.IA_Move"))
  (:Triggered
    (bind _resultvector (CallFunction|GetRotatedForwardCameraVector 0.0 "0.000000,0.000000,1.000000"))
    (Pawn|Input|AddMovementInput _resultvector (* (.y ActionValue) 5e+03) false)
    (bind _resultvector_2 (CallFunction|GetRotatedForwardCameraVector 9e+01 "0.000000,0.000000,1.000000"))
    (Pawn|Input|AddMovementInput _resultvector_2 (* (.x ActionValue) 5e+03) false)
    (CallFunction|DrawDebugVelocityArrow)))

(event Input|EnhancedActionEvents|EnhancedInputActionIA_LookUp
  (params (ActionValue :type Float%20%28double-precision%29) (ElapsedSeconds :type Float%20%28double-precision%29) (TriggeredSeconds :type Float%20%28double-precision%29) (InputAction :type Input%20Action%20Object%20Reference :default "/Game/Input/IA_LookUp.IA_LookUp"))
  (bind _springarm (Variables|Default|GetSpringArm))
  (bind _relativerotation (Variables|/Script/Engine.SceneComponent|GetRelativeRotation _springarm))
  (:Triggered
    (Transformation|SetRelativeRotation (Variables|Default|GetSpringArm) (Math|Rotator|MakeRotator (.roll _relativerotation) (Math|Float|Clamp(Float) (+ (.pitch _relativerotation) ActionValue) -8e+01 -25.0) (.yaw _relativerotation)) false false)))

(event Input|EnhancedActionEvents|EnhancedInputActionIA_TurnAround
  (params (ActionValue :type Float%20%28double-precision%29) (ElapsedSeconds :type Float%20%28double-precision%29) (TriggeredSeconds :type Float%20%28double-precision%29) (InputAction :type Input%20Action%20Object%20Reference :default "/Game/Input/IA_TurnAround.IA_TurnAround"))
  (:Triggered
    (Transformation|AddRelativeRotation (Variables|Default|GetSpringArm) (Math|Rotator|MakeRotator 0.0 0.0 ActionValue) false false)))

(event EventBeginPlay
  (bind _asplayer_controller (Utilities|Casting|CastToPlayerController (Pawn|GetController)))
  (Utilities|IsValid (PlayerController|LocalPlayerSubsystems|GetEnhancedInputLocalPlayerSubsystem _asplayer_controller)
    (:Is%20Valid
      (Input|AddMappingContext (PlayerController|LocalPlayerSubsystems|GetEnhancedInputLocalPlayerSubsystem _asplayer_controller) "/Game/Input/IMC_InputMappingContext.IMC_InputMappingContext" 0 "(bIgnoreAllPressedKeysUntilRelease=True,bForceImmediately=False)")
      (bind _returnvalue (Game|ConstructObjectfromClass (Game|GetPlayerController 0) "/Game/UI/WBP_UI.WBP_UI_C"))
      (bind _output_get (Variables|Default|SetUi _returnvalue))
      (UserInterface|Viewport|AddtoViewport _output_get 0))))

(event Collision|EventHit
  (params (MyComp :type Primitive%20Component%20Object%20Reference) (Other :type Actor%20Object%20Reference) (OtherComp :type Primitive%20Component%20Object%20Reference) (bSelfMoved :type Boolean) (HitLocation :type Vector :default "0, 0, 0") (HitNormal :type Vector :default "0, 0, 0") (NormalImpulse :type Vector :default "0, 0, 0") (Hit :type Hit%20Result%20Structure%20%28by%20ref%29))
  (bind _asbp_target_cube (Utilities|Casting|CastToBP_TargetCube Other))
  (Utilities|FlowControl|Sequence
    (:then_0
      ;[1 1 1] Paint the cube, remove purifier flag
      (Rendering|Material|SetMaterial (Variables|/Game/TargetCube/BP_TargetCube.BP_TargetCube_C|GetCube _asbp_target_cube) 0 (Rendering|Material|GetMaterial (Variables|Default|GetSphere) 0))
      (Variables|/Script/PaintTheCubes.TargetCube|SetbPurifier _asbp_target_cube false)
      (CallFunction|OnHitTargetCube))
    (:then_1
      (Audio|PlaySoundatLocation "/Game/Audio/Pop_11.Pop_11" HitLocation "0, 0, 0" 1.0 1.0 0.0 0 0 0 0)
      (CallFunction|TryEndGame))))

(fn ConstructionScript
  (bind _materialinterface (CallFunction|GetPlayerDefaultColor))
  (Rendering|Material|SetMaterial (Variables|Default|GetSphere) 0 _materialinterface))

(fn GetRotatedForwardCameraVector
  (params (Angle%20Deg :type Float%20%28double-precision%29) (Axis :type Vector :default "0.000000,0.000000,1.000000"))
  (bind _camera (Variables|Default|GetCamera))
  (bind _capsulecomponent (Variables|Default|GetCapsuleComponent))
  (bind _returnvalue (Transformation|GetWorldLocation _capsulecomponent))
  (bind _returnvalue_2 (Transformation|GetWorldLocation _camera))
  (bind _returnvalue_3 (- _returnvalue _returnvalue_2))
  (bind _returnvalue_4 (Math|Vector|RotateVectorAroundAxis (Math|Vector|MakeVector (.x _returnvalue_3) (.y _returnvalue_3) 0.0) Angle%20Deg Axis))
  (return (Math|Vector|MakeVector (.x _returnvalue_4) (.y _returnvalue_4) 0.0)))

(fn DrawDebugVelocityArrow
  (bind _returnvalue (Transformation|GetActorLocation))
  (Rendering|Debug|DrawDebugArrow _returnvalue (+ _returnvalue (Transformation|GetVelocity)) 25.0 "(R=0.150737,G=0.000000,B=1.000000,A=1.000000)" 0.0 1e+01))