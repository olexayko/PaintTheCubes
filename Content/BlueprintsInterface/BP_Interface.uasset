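; BP_Interface is a shared helper library for a cube-painting game, covering default colors and the game-over check.
; Color getters read the player, target and purifier materials from BP_MyGameMode.
; TryEndGame calls EndGame when every BP_TargetCube wears the player material, which shows WBP_LostMenu, switches to UI-only input and pauses.
; GetPurifiers counts the target cubes flagged as purifiers.
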(fn GetPlayerDefaultColor
  (bind _asbp_my_game_mode (CallFunction|GetGamemode (LocalVariables|Get__WorldContext)))
  (return (Variables|/Game/Game/BP_MyGameMode.BP_MyGameMode_C|GetPlayerDefaultMaterial _asbp_my_game_mode)))

(fn GetTargetDefaultColor
  (bind _asbp_my_game_mode (CallFunction|GetGamemode (LocalVariables|Get__WorldContext)))
  (return (Variables|/Game/Game/BP_MyGameMode.BP_MyGameMode_C|GetTargetDefaultMaterial _asbp_my_game_mode)))

(fn GetPurifierDefaultColor
  (bind _asbp_my_game_mode (CallFunction|GetGamemode (LocalVariables|Get__WorldContext)))
  (return (Variables|/Game/Game/BP_MyGameMode.BP_MyGameMode_C|GetPurifierDefaultMaterial _asbp_my_game_mode)))

(fn ShouldEndGame
  (bind ___worldcontext (LocalVariables|Get__WorldContext))
  ;[1 1 1] Search for cubes not painted by the player, return true if found any
  (Utilities|FlowControl|Sequence
    (:then_0
      (bind _materialinterface (CallFunction|GetPlayerDefaultColor ___worldcontext)))
    (:then_1
      (bind _outactors (Actor|GetAllActorsOfClass ___worldcontext "/Game/TargetCube/BP_TargetCube.BP_TargetCube_C"))
      (for _array_element _outactors
        (if (not (== _materialinterface (Rendering|Material|GetMaterial (Variables|/Game/TargetCube/BP_TargetCube.BP_TargetCube_C|GetCube _array_element) 0)))
          (return false)))
      (return true))))

(fn TryEndGame
  (bind ___worldcontext (LocalVariables|Get__WorldContext))
  (bind _should_end_game (CallFunction|ShouldEndGame ___worldcontext))
  (if _should_end_game
    (CallFunction|EndGame ___worldcontext)))

(fn EndGame
  (Utilities|FlowControl|Sequence
    (:then_0
      (LocalVariables|SetPlayerController (Game|GetPlayerController (LocalVariables|Get__WorldContext))))
    (:then_1
      (bind _returnvalue (UserInterface|CreateWidget "/Game/UI/WBP_LostMenu.WBP_LostMenu_C"))
      (UserInterface|Viewport|AddtoViewport _returnvalue 0)
      (Variables|/Script/Engine.PlayerController|SetbShowMouseCursor (LocalVariables|GetPlayerController) true)
      (Input|SetInputModeUIOnly (LocalVariables|GetPlayerController) _returnvalue "DoNotLock" false)
      (Game|SetGamePaused (LocalVariables|Get__WorldContext) true))))

(fn GetGamemode
  (bind _asbp_my_game_mode (Utilities|Casting|CastToBP_MyGameMode (Game|GetGameMode (LocalVariables|Get__WorldContext))))
  (return _asbp_my_game_mode))

(fn GetPurifiers
  (bind _outactors (Actor|GetAllActorsOfClass (LocalVariables|Get__WorldContext) "/Game/TargetCube/BP_TargetCube.BP_TargetCube_C"))
  (for _array_element _outactors
    (if (Variables|/Script/PaintTheCubes.TargetCube|GetbPurifier _array_element)
      (bind _result (Math|Integer|IncrementInt (LocalVariables|GetPurifiers%20Amount)))))
  (return _result))